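; BP_Blocks is an actor that builds a grid of breakable blocks for the ball to destroy.
; The construction script adds a static mesh component at each X/Y cell, driven by the block counts and spaced by Padding.
; On Hit, if the other actor is a BP_Ball, only the struck component is destroyed, so the whole field lives in one actor.
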(event EventBeginPlay)

(event Collision|EventActorBeginOverlap
  (params (OtherActor :type Actor%20Object%20Reference)))

(event EventTick
  (params (DeltaSeconds :type Float%20%28single-precision%29)))

(event Collision|EventHit
  (params (MyComp :type Primitive%20Component%20Object%20Reference) (Other :type Actor%20Object%20Reference) (OtherComp :type Primitive%20Component%20Object%20Reference) (bSelfMoved :type Boolean) (HitLocation :type Vector :default "0, 0, 0") (HitNormal :type Vector :default "0, 0, 0") (NormalImpulse :type Vector :default "0, 0, 0") (Hit :type Hit%20Result%20Structure%20%28by%20ref%29))
  (Utilities|Casting|CastToBP_Ball Other)
  (Components|DestroyComponent MyComp))

(fn ConstructionScript
  (for _index (range 0 (Variables|Default|GetNumbBlockX))
    (for _index_2 (range 0 (Variables|Default|GetNumbBlockY))
      (AddComponent|AddStaticMeshComponent false (Math|Transform|MakeTransform (Math|Vector|MakeVector (Math|Conversions|ToFloat(Integer) (* _index (Variables|Default|GetPadding))) (Math|Conversions|ToFloat(Integer) (* _index_2 (Variables|Default|GetPadding))) 0.0))))))