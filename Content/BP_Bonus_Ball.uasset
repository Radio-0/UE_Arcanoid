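; BP_Bonus_Ball is a bonus ball actor that moves on its own and bounces off blocking surfaces.
; Each Tick it makes a swept move along DirectionBonus at SpeedBonus, scaled by delta time.
; On a blocking hit, GetReflectionVector computes the new direction from the current one and the hit normal's X and Y.
; Overlapping a KillZVolume destroys the ball.
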(event EventBeginPlay)

(event Collision|EventActorBeginOverlap
  (params (OtherActor :type Actor%20Object%20Reference))
  (Utilities|Casting|CastToKillZVolume OtherActor)
  (Actor|DestroyActor))

(event EventTick
  (params (DeltaSeconds :type Float%20%28single-precision%29))
  (bind _sweephitresult (Transformation|AddActorWorldOffset (* (* (Variables|Default|GetDirectionBonus) (Variables|Default|GetSpeedBonus)) DeltaSeconds) true))
  (if (.bBlockingHit (Collision|BreakHitResult _sweephitresult))
    (Variables|Default|SetDirectionBonus (Math|Vector|GetReflectionVector (Variables|Default|GetDirectionBonus) (Math|Vector|MakeVector (.X (Math|Vector|BreakVector (.Normal (Collision|BreakHitResult _sweephitresult)))) (.Y (Math|Vector|BreakVector (.Normal (Collision|BreakHitResult _sweephitresult)))) 0.0)))))

(fn ConstructionScript)